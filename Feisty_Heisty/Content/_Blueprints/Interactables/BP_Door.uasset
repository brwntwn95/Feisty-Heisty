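; Interactable door that swings open when BP_Player enters its Box trigger and closes when the player leaves.
; A timeline drives the Door's relative yaw, playing to open and reversing to close, despite the "Slide" event names.
; Door collision switches off as opening starts and back on as closing starts, each with a sound at the door's location.
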(event `Slide Door Open`
  (bind _door (`self.Door`))
  ;[1 1 1] Slides Wall on Z axis relative to its location when activated
  (`PrimitiveComponent.SetCollisionEnabled` _door "NoCollision")
  (`GameplayStatics.SpawnSoundAtLocation` "/Game/_Sounds/Doors/Door_Open.Door_Open" (`SceneComponent.K2_GetComponentLocation` _door) (struct) 0.2 1.0 0.0 null null)
  (bind (_direction _newtrack_0) (`Timeline|Timeline_1` :!label _label)
    (:`Update`
      (`SceneComponent.K2_SetRelativeRotation` (`self.Door`) (`KismetMathLibrary.MakeRotator` 0.0 0.0 _newtrack_0) false false))))

(event `Slide Door Closed`
  (bind _door (`self.Door`))
  ;[1 1 1] Slides Wall on Z axis relative to its location when activated
  (`PrimitiveComponent.SetCollisionEnabled` _door "QueryAndPhysics")
  (`GameplayStatics.SpawnSoundAtLocation` "/Game/_Sounds/Doors/Door_Close.Door_Close" (`SceneComponent.K2_GetComponentLocation` _door) (struct) 0.2 1.0 0.0 null null)
  (goto _label :!via `Reverse`))

(event `self.Box.OnComponentBeginOverlap`
  (params (OverlappedComponent :type "PrimitiveComponent Object Reference") (OtherActor :type "Actor Object Reference") (OtherComp :type "PrimitiveComponent Object Reference") (OtherBodyIndex :type Integer) (bFromSweep :type Boolean) (SweepResult :type "HitResult Structure (by ref)"))
  (cast `/Game/_Blueprints/Player/BP_Player` OtherActor)
  (`self.Slide Door Open`))

(event `self.Box.OnComponentEndOverlap`
  (params (OverlappedComponent :type "PrimitiveComponent Object Reference") (OtherActor :type "Actor Object Reference") (OtherComp :type "PrimitiveComponent Object Reference") (OtherBodyIndex :type Integer))
  (cast `/Game/_Blueprints/Player/BP_Player` OtherActor)
  (`self.Slide Door Closed`))

(fn `UserConstructionScript`)