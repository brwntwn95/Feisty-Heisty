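; BP_EndGame is an interactable trigger that ends the game when BP_Player overlaps its Box.
; On overlap it hides the player, disables movement, mutes the Music sound class and plays the EndSequence level sequence.
; After a fixed delay, rather than a sequence-finished event, it shows the UI_EndLevel widget pointed at MainMenu, pauses the game, shows the cursor and restores music volume.
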(event `self.Box.OnComponentBeginOverlap`
  (params (OverlappedComponent :type "PrimitiveComponent Object Reference") (OtherActor :type "Actor Object Reference") (OtherComp :type "PrimitiveComponent Object Reference") (OtherBodyIndex :type Integer) (bFromSweep :type Boolean) (SweepResult :type "HitResult Structure (by ref)"))
  (bind _asbp_player (cast `/Game/_Blueprints/Player/BP_Player` OtherActor))
  (`self.SetActorHiddenInGame` _asbp_player true)
  (`CharacterMovementComponent.DisableMovement` (`Character.CharacterMovement` _asbp_player))
  (`GameplayStatics.SetSoundMixClassOverride` "/Game/_Sounds/Mix/MasterSoundClassMix.MasterSoundClassMix" "/Engine/EngineSounds/Music.Music" 0.0 1.0 0.0)
  (bind (_outactor _returnvalue) (`LevelSequencePlayer.CreateLevelSequencePlayer` "/Game/_LevelSequence/EndSequence.EndSequence"))
  (`MovieSceneSequencePlayer.Play` _returnvalue)
  (`KismetSystemLibrary.Delay` 14.9)
  (bind _returnvalue_2 (`|CreateWidget` "/Game/_UI/UI_EndLevel.UI_EndLevel_C" null "MainMenu"))
  (`UserWidget.AddToViewport` _returnvalue_2 0)
  (`GameplayStatics.SetGamePaused` true)
  (set `PlayerController.bShowMouseCursor` true (`GameplayStatics.GetPlayerController` 0))
  (`GameplayStatics.SetSoundMixClassOverride` "/Game/_Sounds/Mix/MasterSoundClassMix.MasterSoundClassMix" "/Engine/EngineSounds/Music.Music" 1.0 1.0 0.0))

(fn `UserConstructionScript`)