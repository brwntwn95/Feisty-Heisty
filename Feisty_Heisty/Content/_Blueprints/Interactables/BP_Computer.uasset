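; Hackable computer that the player hacks by holding Interact inside its trigger box, opening linked doors and powering a wire.
; Box overlap toggles input, the UI_Hack widget and a gate; a retriggerable delay completes the hack if Interact is still held.
; A self-recalling Delay loop feeds timer elapsed time to the hold bar.
; Tick updates the locked screen and, once hacked, repeatedly disables input and removes the widget.
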(event `self.ReceiveTick`
  (params (DeltaSeconds :type "Float (single-precision)"))
  (bind _widgetref (`self.WidgetRef`))
  (`|ExecutionSequence`
    (:`then_0`
      (if (`self.isHacked?`)
        (`self.DisableInput` (`GameplayStatics.GetPlayerController` 0))
        (`Widget.RemoveFromParent` _widgetref)
        (set `/Game/_UI/UI_Hack.MaxTimeHeld` 0.0 _widgetref)))
    (:`then_1`
      (if (`self.canBeHacked`)
        (`SceneComponent.SetVisibility` (`self.LockedScreen`) true false)
        (else
          (`SceneComponent.SetVisibility` (`self.LockedScreen`) false false :!label _label))))
    (:`then_2`
      (if (`self.isHacked?`)
        (goto _label)))))

(event `InputAction|Interact`
  (params (Key :type "Key Structure"))
  (bind _canbehacked (`self.canBeHacked`))
  (:`Pressed`
    (if _canbehacked
      (set `self.IsHeld?` true)
      (`/Engine/EditorBlueprintResources/StandardMacros.Gate` true :!label _label_2
        (:`Exit`
          (`|ExecutionSequence`
            (:`then_0`
              (`KismetSystemLibrary.RetriggerableDelay` (`self.MaxHoldTime`))
              (if (`self.IsHeld?`)
                (set `self.IsHacked?` true)
                (set `self.canBeHacked` false)
                (`/Engine/EditorBlueprintResources/StandardMacros.DoOnce` false :!label _label_3
                  (:`Completed`
                    (`GameplayStatics.SpawnSoundAtLocation` "/Game/_Sounds/Hacking/Complete/Hack_Complete_2.Hack_Complete_2" (0.0 0.0 0.0) (struct) 0.2 1.0 0.0 null null)
                    (`/Game/_Blueprints/Interactables/BP_Gate.Slide Door Open` (`self.GateRef`))
                    (`/Game/_Blueprints/Interactables/BP_WireSpline.Powered` (`self.Wire`))
                    (`/Game/_Blueprints/Interactables/BP_DoubleDoor.Slide Door Open` (`self.DoorOpen`))
                    (`SceneComponent.SetVisibility` (`self.HackedScreen`) true false)))))
            (:`then_1`
              (`self.Timer`)
              (`self.Update Timer`)))))))
  (:`Released`
    (if _canbehacked
      (set `self.IsHeld?` false))))

(event `self.Box.OnComponentBeginOverlap`
  (params (OverlappedComponent :type "PrimitiveComponent Object Reference") (OtherActor :type "Actor Object Reference") (OtherComp :type "PrimitiveComponent Object Reference") (OtherBodyIndex :type Integer) (bFromSweep :type Boolean) (SweepResult :type "HitResult Structure (by ref)"))
  (bind _returnvalue (`GameplayStatics.GetPlayerController` 0))
  (bind _widgetref (`self.WidgetRef`))
  (cast `/Game/_Blueprints/Player/BP_Player` OtherActor)
  (if (`self.canBeHacked`)
    (`self.EnableInput` _returnvalue)
    (`UserWidget.AddToViewport` _widgetref 0)
    (set `/Game/_UI/UI_Hack.MaxTimeHeld` (`self.MaxHoldTime`) _widgetref)
    (if (`self.IsHacked?`)
      (`self.DisableInput` _returnvalue (`GameplayStatics.GetPlayerController` 0))
      (`Widget.RemoveFromParent` (`self.WidgetRef`))
      (goto _label_3)
      (else
        (goto _label_2 :!via `Open`)))))

(event `self.Box.OnComponentEndOverlap`
  (params (OverlappedComponent :type "PrimitiveComponent Object Reference") (OtherActor :type "Actor Object Reference") (OtherComp :type "PrimitiveComponent Object Reference") (OtherBodyIndex :type Integer))
  (cast `/Game/_Blueprints/Player/BP_Player` OtherActor)
  (if (`self.canBeHacked`)
    (`self.DisableInput` (`GameplayStatics.GetPlayerController` 0))
    (`Widget.RemoveFromParent` (`self.WidgetRef`))
    (if (`self.IsHacked?`)
      (`self.DisableInput` (`GameplayStatics.GetPlayerController` 0))
      (`Widget.RemoveFromParent` (`self.WidgetRef`))
      (else
        (goto _label_2 :!via `Close`)))))

(event `self.ReceiveBeginPlay`
  (bind _returnvalue (`|CreateWidget` "/Game/_UI/UI_Hack.UI_Hack_C" (`GameplayStatics.GetPlayerController` 0)))
  (set `self.WidgetRef` _returnvalue))

(event `Stop Timer`
  ;[1 1 1] Update Hacking Bar
  (`KismetSystemLibrary.K2_PauseTimerHandle` (stale `Timer` _returnvalue)))

(event `Timer`
  ;[1 1 1] Update Hacking Bar
  (bind _returnvalue (`KismetSystemLibrary.K2_SetTimerDelegate` (delegate `Timer`) (`self.MaxHoldTime`))))

(event `Update Timer`
  (bind _widgetref (`self.WidgetRef`))
  ;[1 1 1] Update Hacking Bar
  (if (`self.IsHeld?`)
    (set `/Game/_UI/UI_Hack.TimeHeld` (`KismetSystemLibrary.K2_GetTimerElapsedTimeHandle` (stale `Timer` _returnvalue)) _widgetref)
    (else
      (`self.Stop Timer`)
      (set `/Game/_UI/UI_Hack.TimeHeld` 0.0 _widgetref)))
  (`KismetSystemLibrary.Delay` 0.005)
  (`self.Update Timer`))

(fn `UserConstructionScript`)