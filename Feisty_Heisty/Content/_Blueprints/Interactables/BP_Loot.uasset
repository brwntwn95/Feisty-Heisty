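; BP_Loot is a collectible pickup that floats in place and awards score to the player.
; A Float timeline, re-triggered from Tick, drives the mesh's relative height.
; Sphere overlap with BP_Player plays a coin sound, increments the player's Score and destroys the actor.
; BeginPlay sets the mesh and, after a delay, makes a one-time ObjectsPickedUp check for extra sounds; that counter increments on any actor overlap.
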(event `self.ReceiveBeginPlay`
  (`StaticMeshComponent.SetStaticMesh` (`self.Mesh`) (`self.New Mesh`))
  (`KismetSystemLibrary.Delay` 2.0)
  (if (== (`self.Objects Picked Up`) (`KismetMathLibrary.RandomIntegerInRange` 1 2))
    (`GameplayStatics.PlaySoundAtLocation` "/Game/_Sounds/Pick_Up_Dialogue/Pick_Up.Pick_Up" (`self.K2_GetActorLocation`) (struct) 1.0 1.0 0.0 null null null null)
    (if (== (`self.Objects Picked Up`) (`self.Total Objects`))
      (`GameplayStatics.PlaySoundAtLocation` "/Game/_Sounds/Pick_Up_Dialogue/Half_Down_Cue.Half_Down_Cue" (`self.K2_GetActorLocation`) (struct) 1.0 1.0 0.0 null null null null))))

(event `self.ReceiveActorBeginOverlap`
  (params (OtherActor :type "Actor Object Reference"))
  (set `self.Objects Picked Up` (+ (`self.Objects Picked Up`) 1)))

(event `self.ReceiveTick`
  (params (DeltaSeconds :type "Float (single-precision)"))
  (bind (_direction _newtrack_0) (`Timeline|Float`)
    (:`Update`
      (`SceneComponent.K2_SetRelativeLocation` (`self.Mesh`) (`KismetMathLibrary.MakeVector` 0.0 0.0 (.z _newtrack_0)) false false))))

(event `self.Sphere.OnComponentBeginOverlap`
  (params (OverlappedComponent :type "PrimitiveComponent Object Reference") (OtherActor :type "Actor Object Reference") (OtherComp :type "PrimitiveComponent Object Reference") (OtherBodyIndex :type Integer) (bFromSweep :type Boolean) (SweepResult :type "HitResult Structure (by ref)"))
  (bind _asbp_player (cast `/Game/_Blueprints/Player/BP_Player` OtherActor))
  (`GameplayStatics.PlaySound2D` "/Game/_Sounds/Loot/Coins.Coins" 1.0 1.0 0.0 null null)
  (set `/Game/_Blueprints/Player/BP_Player.Score` (+ (`/Game/_Blueprints/Player/BP_Player.Score` _asbp_player) 1) _asbp_player)
  (`self.K2_DestroyActor`))

(fn `UserConstructionScript`)