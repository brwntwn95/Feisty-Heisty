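; BP_LoadLevel is an interactable trigger that ends the current level when BP_Player overlaps its box.
; The overlap disables player movement, plays the FadeOut level sequence, then after a short delay adds a UI_EndLevel widget to the viewport, passing it LevelName.
; It then pauses the game and shows the mouse cursor; the actor itself does no level loading.
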(event `self.Box.OnComponentBeginOverlap`
  (params (OverlappedComponent :type "PrimitiveComponent Object Reference") (OtherActor :type "Actor Object Reference") (OtherComp :type "PrimitiveComponent Object Reference") (OtherBodyIndex :type Integer) (bFromSweep :type Boolean) (SweepResult :type "HitResult Structure (by ref)"))
  (bind _asbp_player (cast `/Game/_Blueprints/Player/BP_Player` OtherActor))
  (`CharacterMovementComponent.DisableMovement` (`Character.CharacterMovement` _asbp_player))
  (bind (_outactor _returnvalue) (`LevelSequencePlayer.CreateLevelSequencePlayer` "/Game/_LevelSequence/FadeOut.FadeOut"))
  (`MovieSceneSequencePlayer.Play` _returnvalue)
  (`KismetSystemLibrary.Delay` 2.0)
  (bind _returnvalue_2 (`|CreateWidget` "/Game/_UI/UI_EndLevel.UI_EndLevel_C" null (`self.Level Name`)))
  (`UserWidget.AddToViewport` _returnvalue_2 0)
  (`GameplayStatics.SetGamePaused` true)
  (set `PlayerController.bShowMouseCursor` true (`GameplayStatics.GetPlayerController` 0)))

(fn `UserConstructionScript`)