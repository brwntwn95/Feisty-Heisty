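; BP_Camera is a security camera that sweeps side to side and catches the player within its view.
; RotateCam loops from BeginPlay, using a FlipFlop to alternate the yaw offset between LowRot and MaxRot for each timed MoveComponentTo.
; Tick approximates a view cone with eight stationary sphere traces of geometrically growing radius along the forward vector.
; A player hit calls PlayerCaught and plays an alarm sound, only once through DoOnce.
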(event `self.ReceiveTick`
  (params (DeltaSeconds :type "Float (single-precision)"))
  ;[1 1 1] Camera View Cone
  (set `self.Current Start Location` (`self.K2_GetActorLocation`))
  (for _ (range 8)
    (bind _output_get (set `self.Diameter` (* (`self.Diameter`) 2.47)))
    (bind _output_get_2 (set `self.Current Start Location` (+ (`self.Current Start Location`) (* (`self.GetActorForwardVector`) (/ (`self.Diameter`) 2.0)))))
    (bind _outhit (`KismetSystemLibrary.SphereTraceSingle` _output_get_2 _output_get_2 (/ _output_get 4.0) "TraceTypeQuery1"))
    (bind _asbp_player (cast `/Game/_Blueprints/BP_Player` (`.HitActor` (`GameplayStatics.BreakHitResult` _outhit))))
    (`/Engine/EditorBlueprintResources/StandardMacros.DoOnce` false
      (:`Completed`
        (`/Game/_Blueprints/BP_Player.Player Caught` _asbp_player)
        (`GameplayStatics.PlaySoundAtLocation` "/Game/_Sounds/Alarms/Camera_Alarm_Cue.Camera_Alarm_Cue" (`SceneComponent.K2_GetComponentLocation` (`self.CameraMesh`)) (struct) 0.8 1.0 0.0 null null null null))))
  (set `self.Current Start Location` (0.0 0.0 0.0))
  (set `self.Diameter` 0.4))

(event `self.ReceiveBeginPlay`
  ;[1 1 1] Camera View Cone
  (`self.Rotate Cam`))

(event `Rotate Cam`
  (bind _defaultsceneroot (`self.DefaultSceneRoot`))
  (bind (_returnvalue_roll _returnvalue_pitch _returnvalue_yaw) (`KismetMathLibrary.BreakRotator` (`SceneComponent.K2_GetComponentRotation` _defaultsceneroot)))
  ;[1 1 1] Rotate Camera
  (`/Engine/EditorBlueprintResources/StandardMacros.FlipFlop` :!label _label
    (:`A`
      (set `self.Reached One of the sides` true))
    (:`B`
      (set `self.Reached One of the sides` false)))
  (`KismetSystemLibrary.MoveComponentTo` _defaultsceneroot (`SceneComponent.K2_GetComponentLocation` _defaultsceneroot) (`KismetMathLibrary.MakeRotator` _returnvalue_roll _returnvalue_pitch (+ _returnvalue_yaw (`KismetMathLibrary.SelectFloat` (`self.Low Rot`) (`self.Max Rot`) (`self.Reached One of the sides`)))) false false (`self.Rot Speed`) true)
  (goto _label))

(fn `UserConstructionScript`)