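; Test AI pawn that patrols between two locations, pausing at each, and displays a vision cone.
; Each tick it runs the VisionCone EQS query and converts the results into actor-relative, flattened triangle-fan vertices for a procedural mesh.
; Tick also casts a forward chain of growing sphere traces, whose results go unused.
; The caught sound and arrow-based multi-sphere traces are disconnected, so no detection response runs.
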(event `self.ReceiveTick`
  (params (DeltaSeconds :type "Float (single-precision)"))
  (`|ExecutionSequence`
    (:`then_0`
      (bind _returnvalue (`EnvQueryManager.RunEQSQuery` "/Game/_Blueprints/Enemies/VisionCone.VisionCone" self "AllMatching"))
      (add `EnvQueryInstanceBlueprintWrapper.OnQueryFinishedEvent` _returnvalue (delegate `Make Cone`)))
    (:`then_1`
      (set `self.Current Start Location` (`self.K2_GetActorLocation`))
      (for _ (range 4)
        (bind _output_get (set `self.Diameter` (* (`self.Diameter`) 1.87)))
        (bind _output_get_2 (set `self.Current Start Location` (+ (`self.Current Start Location`) (* (`self.GetActorForwardVector`) (/ (`self.Diameter`) 4.0)))))
        (`KismetSystemLibrary.SphereTraceSingle` _output_get_2 _output_get_2 (/ _output_get 3.0) "TraceTypeQuery1"))
      (set `self.Current Start Location` (0.0 0.0 0.0))
      (set `self.Diameter` 50.0))))

(event `Make Cone`
  (params (QueryInstance :type "EnvQueryInstanceBlueprintWrapper Object Reference") (QueryStatus :type "EEnvQueryStatus Enum" :default "Processing"))
  (bind _resultlocations (`EnvQueryInstanceBlueprintWrapper.GetQueryResultsAsLocations` QueryInstance))
  (bind _output_get (set `self.SightPoints` _resultlocations))
  (bind (_vertices _triangles) (`self.ConvertSightPointsToVertices` _output_get))
  (`self.MakeTheCone` _vertices _triangles))

(event `self.ReceiveBeginPlay`
  (`KismetArrayLibrary.Array_Resize` (`self.Vertices`) (`self.+1 EQS Points`))
  ;[1 1 1] AI Move Location, wait, Move to new location
  (`|AIMoveTo` self (`self.Loc1`) null :!label _label
    (:`OnSuccess`
      (`KismetSystemLibrary.Delay` (`self.Pause`))
      (`|AIMoveTo` self (`self.Loc2`) null
        (:`OnSuccess`
          (`KismetSystemLibrary.Delay` (`self.Pause`))
          (goto _label))))))

(fn `ConvertSightPointsToVertices`
  (params (SightPoints :type "Array of Vector Structure"))
  (returns (Vertices :type "Array of Vector Structure") (Triangles :type "Array of Integer"))
  (bind _returnvalue (`KismetArrayLibrary.Array_Length` (`self.Vertices`)))
  (`KismetArrayLibrary.Array_Set` (`self.Vertices`))
  (for (_array_element _array_index) SightPoints
    (`KismetArrayLibrary.Array_Set` (`self.Vertices`) (+ _array_index 1) (`KismetMathLibrary.MakeVector` (- (.x _array_element) (.x (`self.K2_GetActorLocation`))) (- (.y _array_element) (.y (`self.K2_GetActorLocation`))))))
  (`KismetArrayLibrary.Array_Resize` (`self.Triangles`) (* _returnvalue 3))
  (for _index (range (+ _returnvalue 1))
    (bind _returnvalue_2 (* _index 3))
    (`KismetArrayLibrary.Array_Set` (`self.Triangles`) _returnvalue_2)
    (bind _returnvalue_3 (+ _returnvalue_2 1))
    (bind _returnvalue_4 (+ _index 1))
    (`KismetArrayLibrary.Array_Set` (`self.Triangles`) _returnvalue_3 _returnvalue_4)
    (`KismetArrayLibrary.Array_Set` (`self.Triangles`) (+ _returnvalue_3 1) (+ _returnvalue_4 1)))
  (return (`self.Vertices`) (`self.Triangles`)))

(fn `MakeTheCone`
  (params (Vertices :type "Array of Vector Structure") (Triangles :type "Array of Integer"))
  (bind _visioncone (`self.VisionCone`))
  (`ProceduralMeshComponent.CreateMeshSection_LinearColor` :`self` _visioncone :`Vertices` Vertices :`Triangles` Triangles)
  (`PrimitiveComponent.SetMaterial` _visioncone 0 "/Game/_Materials/M_Cone_Inst.M_Cone_Inst")
  (`SceneComponent.K2_SetWorldRotation` :`self` _visioncone))

(fn `UserConstructionScript`)