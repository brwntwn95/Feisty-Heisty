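; Test Blueprint of a hackable computer, meant to open a gate and power a wire after a hold-to-hack interaction.
; A gated retriggerable delay checks the hold and sets IsHacked.
; A recursive short-delay loop feeds timer progress to the UI_Hack widget and plays the interact sound.
; The overlap events are empty, and the casts, widget setup and hold logic sit in unconnected chains that never run.
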(event `InputAction|Interact`
  (params (Key :type "Key Structure")))

(event `self.Box.OnComponentBeginOverlap`
  (params (OverlappedComponent :type "PrimitiveComponent Object Reference") (OtherActor :type "Actor Object Reference") (OtherComp :type "PrimitiveComponent Object Reference") (OtherBodyIndex :type Integer) (bFromSweep :type Boolean) (SweepResult :type "HitResult Structure (by ref)")))

(event `self.Box.OnComponentEndOverlap`
  (params (OverlappedComponent :type "PrimitiveComponent Object Reference") (OtherActor :type "Actor Object Reference") (OtherComp :type "PrimitiveComponent Object Reference") (OtherBodyIndex :type Integer)))

(event `Stop Timer`
  ;[1 1 1] Update Hacking Bar
  (`KismetSystemLibrary.K2_PauseTimerHandle` (stale `Timer` _returnvalue)))

(event `Timer`
  ;[1 1 1] Update Hacking Bar
  (bind _returnvalue (`KismetSystemLibrary.K2_SetTimerDelegate` (delegate `Timer`) (`self.MaxHoldTime`))))

(event `Update Timer`
  (bind _widgetref (`self.WidgetRef`))
  ;[1 1 1] Update Hacking Bar
  (if (`self.IsHeld?`)
    (`GameplayStatics.PlaySound2D` "/Game/_Sounds/Hacking/Interact/Computer_Interact.Computer_Interact" 1.0 1.0 0.0 null null)
    (set `/Game/_UI/UI_Hack.TimeHeld` (`KismetSystemLibrary.K2_GetTimerElapsedTimeHandle` (stale `Timer` _returnvalue)) _widgetref)
    (else
      (`self.Stop Timer`)
      (set `/Game/_UI/UI_Hack.TimeHeld` 0.0 _widgetref)))
  (`KismetSystemLibrary.Delay` 0.005)
  (`self.Update Timer`))

(fn `UserConstructionScript`)