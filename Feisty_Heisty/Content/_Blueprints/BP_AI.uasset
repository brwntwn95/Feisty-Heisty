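; Guard AI that patrols between two locations with pauses and catches the player on sight.
; Each tick, an EQS query supplies points that become a procedural triangle-fan mesh showing the vision cone.
; Separately, five fanned forward sphere traces detect BP_Player and call PlayerCaught, gated by DoOnce nodes.
; A shared catch reaction plays rifle montages and a sound, moves to the player, then resets detection and resumes patrol.
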(event `AI Pathing`
  ;[0.3118 0.9701 1] Begin Play, Resize Vertices Array to Match EQS Points +1 then begin moving to locations on loop
  ;;[0.5141 1 0.5219] AI Move Location, wait, Move to new location
  (`|AIMoveTo` self (`self.Loc1`) null :!label _label
    (:`OnSuccess`
      (`KismetSystemLibrary.Delay` (`self.Pause`))
      (`|AIMoveTo` self (`self.Loc2`) null
        (:`OnSuccess`
          (`KismetSystemLibrary.Delay` (`self.Pause`))
          (goto _label))))))

(event `self.ReceiveBeginPlay`
  ;[0.3118 0.9701 1] Begin Play, Resize Vertices Array to Match EQS Points +1 then begin moving to locations on loop
  (`KismetArrayLibrary.Array_Resize` (`self.Vertices`) (`self.+1 EQS Points`))
  (`self.AI Pathing`))

(event `self.ReceiveTick`
  (params (DeltaSeconds :type "Float (single-precision)"))
  (bind _capsulecomponent (`self.CapsuleComponent`))
  (bind _radius (`self.Radius`))
  (bind _returnvalue (`SceneComponent.K2_GetComponentLocation` _capsulecomponent))
  (bind _returnvalue_2 (`SceneComponent.GetForwardVector` _capsulecomponent))
  (bind _returnvalue_3 (+ _returnvalue _returnvalue_2))
  (`|ExecutionSequence`
    (:`then_0`
      ;[1 0.9866 0.3783] Create View Cone
      (bind _returnvalue_4 (`EnvQueryManager.RunEQSQuery` "/Game/_Blueprints/VisionCone.VisionCone" self "AllMatching"))
      (add `EnvQueryInstanceBlueprintWrapper.OnQueryFinishedEvent` _returnvalue_4 (delegate `Make Cone`)))
    (:`then_1`
      ;[1 0.5336 0.4638] Sphere Traces to Detect Player
      (bind _outhits (`KismetSystemLibrary.SphereTraceMulti` _returnvalue (+ _returnvalue_3 (* _returnvalue_2 (`self.Range`))) _radius "TraceTypeQuery1" true))
      (for _array_element _outhits
        (bind _asbp_player (cast `/Game/_Blueprints/BP_Player` (`.HitActor` (`GameplayStatics.BreakHitResult` _array_element))))
        (`/Engine/EditorBlueprintResources/StandardMacros.DoOnce` false :!label _label_2
          (:`Completed`
            (`/Game/_Blueprints/BP_Player.Player Caught` _asbp_player)
            (`/Engine/EditorBlueprintResources/StandardMacros.DoOnce` false :!label _label_3
              (:`Completed`
                (bind _returnvalue_5 (`self.PlayAnimMontage` "/Game/_Animation/Guard/GuardRifleDownMont.GuardRifleDownMont"))
                (`self.PlayAnimMontage` "/Game/_Animation/Guard/Guard_Rifle_Up_Mont.Guard_Rifle_Up_Mont" _returnvalue_5)
                (`GameplayStatics.PlaySoundAtLocation` "/Game/_Sounds/Player_Caught/Player_Caught.Player_Caught" (`SceneComponent.K2_GetComponentLocation` (`self.CapsuleComponent`)) (struct) 0.8 1.0 0.0 null null null null)
                (`|AIMoveTo` self (`SceneComponent.K2_GetComponentLocation` (`Actor.RootComponent` (`GameplayStatics.GetPlayerCharacter` 0))) (stale _asbp_player_3) 10.0
                  (:`then`
                    (`KismetSystemLibrary.Delay` 3.0)
                    (`self.ResetAI`)
                    (`self.AI Pathing`)))))))))
    (:`then_2`
      (bind _outhits_2 (`KismetSystemLibrary.SphereTraceMulti` _returnvalue (+ _returnvalue_3 (* (`KismetMathLibrary.GreaterGreater_VectorRotator` _returnvalue_2 (struct :`Yaw` 30.0)) (`self.Range`))) _radius "TraceTypeQuery1" true))
      (for _array_element_2 _outhits_2
        (bind _asbp_player_2 (cast `/Game/_Blueprints/BP_Player` (`.HitActor` (`GameplayStatics.BreakHitResult` _array_element_2))))
        (`/Engine/EditorBlueprintResources/StandardMacros.DoOnce` false :!label _label_4
          (:`Completed`
            (`/Game/_Blueprints/BP_Player.Player Caught` _asbp_player_2)
            (goto _label_3)))))
    (:`then_3`
      (bind _outhits_3 (`KismetSystemLibrary.SphereTraceMulti` _returnvalue (+ _returnvalue_3 (* (`KismetMathLibrary.GreaterGreater_VectorRotator` _returnvalue_2 (struct :`Yaw` -30.0)) (`self.Range`))) _radius "TraceTypeQuery1" true))
      (for _array_element_3 _outhits_3
        (bind _asbp_player_3 (cast `/Game/_Blueprints/BP_Player` (`.HitActor` (`GameplayStatics.BreakHitResult` _array_element_3))))
        (`/Engine/EditorBlueprintResources/StandardMacros.DoOnce` false :!label _label_5
          (:`Completed`
            (`/Game/_Blueprints/BP_Player.Player Caught` _asbp_player_3)
            (goto _label_3)))))
    (:`then_4`
      (bind _outhits_4 (`KismetSystemLibrary.SphereTraceMulti` _returnvalue (+ _returnvalue_3 (* (`KismetMathLibrary.GreaterGreater_VectorRotator` _returnvalue_2 (struct :`Yaw` -15.0)) (`self.Range`))) _radius "TraceTypeQuery1" true))
      (for _array_element_4 _outhits_4
        (bind _asbp_player_4 (cast `/Game/_Blueprints/BP_Player` (`.HitActor` (`GameplayStatics.BreakHitResult` _array_element_4))))
        (`/Engine/EditorBlueprintResources/StandardMacros.DoOnce` false :!label _label_6
          (:`Completed`
            (`/Game/_Blueprints/BP_Player.Player Caught` _asbp_player_4)
            (goto _label_3)))))
    (:`then_5`
      (bind _outhits_5 (`KismetSystemLibrary.SphereTraceMulti` _returnvalue (+ _returnvalue_3 (* (`KismetMathLibrary.GreaterGreater_VectorRotator` _returnvalue_2 (struct :`Yaw` 15.0)) (`self.Range`))) _radius "TraceTypeQuery1" true))
      (for _array_element_5 _outhits_5
        (bind _asbp_player_5 (cast `/Game/_Blueprints/BP_Player` (`.HitActor` (`GameplayStatics.BreakHitResult` _array_element_5))))
        (`/Engine/EditorBlueprintResources/StandardMacros.DoOnce` false :!label _label_7
          (:`Completed`
            (`/Game/_Blueprints/BP_Player.Player Caught` _asbp_player_5)
            (goto _label_3)))))))

(event `Make Cone`
  (params (QueryInstance :type "EnvQueryInstanceBlueprintWrapper Object Reference") (QueryStatus :type "EEnvQueryStatus Enum" :default "Processing"))
  ;[1 0.9866 0.3783] Create View Cone
  (bind _resultlocations (`EnvQueryInstanceBlueprintWrapper.GetQueryResultsAsLocations` QueryInstance))
  (bind _output_get (set `self.SightPoints` _resultlocations))
  (bind (_vertices _triangles) (`self.ConvertSightPointsToVertices` _output_get))
  (`self.MakeTheCone` _vertices _triangles))

(event `ResetAI`
  ;[1 0.5336 0.4638] Sphere Traces to Detect Player
  (`|ExecutionSequence`
    (:`then_0`
      (goto _label_2 :!via `Reset`))
    (:`then_1`
      (goto _label_4 :!via `Reset`))
    (:`then_2`
      (goto _label_5 :!via `Reset`))
    (:`then_3`
      (goto _label_6 :!via `Reset`))
    (:`then_4`
      (goto _label_7 :!via `Reset`))
    (:`then_5`
      (goto _label_3 :!via `Reset`))))

(fn `ConvertSightPointsToVertices`
  (params (SightPoints :type "Array of Vector Structure"))
  (returns (Vertices :type "Array of Vector Structure") (Triangles :type "Array of Integer"))
  (bind _returnvalue (`KismetArrayLibrary.Array_Length` (`self.Vertices`)))
  (`KismetArrayLibrary.Array_Set` (`self.Vertices`))
  (for (_array_element _array_index) SightPoints
    (`KismetArrayLibrary.Array_Set` (`self.Vertices`) (+ _array_index 1) (`KismetMathLibrary.MakeVector` (- (.x _array_element) (.x (`self.K2_GetActorLocation`))) (- (.y _array_element) (.y (`self.K2_GetActorLocation`))))))
  (`KismetArrayLibrary.Array_Resize` (`self.Triangles`) (* _returnvalue 3))
  (for _index (range (+ _returnvalue 1))
    (bind _returnvalue_2 (* _index 3))
    (`KismetArrayLibrary.Array_Set` (`self.Triangles`) _returnvalue_2)
    (bind _returnvalue_3 (+ _returnvalue_2 1))
    (bind _returnvalue_4 (+ _index 1))
    (`KismetArrayLibrary.Array_Set` (`self.Triangles`) _returnvalue_3 _returnvalue_4)
    (`KismetArrayLibrary.Array_Set` (`self.Triangles`) (+ _returnvalue_3 1) (+ _returnvalue_4 1)))
  (return (`self.Vertices`) (`self.Triangles`)))

(fn `MakeTheCone`
  (params (Vertices :type "Array of Vector Structure") (Triangles :type "Array of Integer"))
  (bind _visioncone (`self.VisionCone`))
  (`ProceduralMeshComponent.CreateMeshSection_LinearColor` :`self` _visioncone :`Vertices` Vertices :`Triangles` Triangles)
  (`PrimitiveComponent.SetMaterial` _visioncone 0 "/Game/_Materials/M_Cone_Inst.M_Cone_Inst")
  (`SceneComponent.K2_SetWorldRotation` :`self` _visioncone))

(fn `UserConstructionScript`)