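; BP_Laser_Hayden is a laser actor apparently meant to rotate and detect the player, but its Tick event is empty.
; Disconnected nodes would play a running sound, line trace forward from an Arrow component and yaw the actor by RotationSpeed.
; A separate unwired DoOnce prints a hit message and resets after a delay, and the trace's hit result is unused.
; None of this logic runs, and the construction script is empty.
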(event `self.ReceiveTick`
  (params (DeltaSeconds :type "Float (single-precision)"))
  ;[1 0.7067 0.6868] Draws a line and detects if player was hit
)

(fn `UserConstructionScript`)