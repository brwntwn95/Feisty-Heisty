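; BP_Respawn is a checkpoint trigger that sets where the player respawns.
; When BP_Player overlaps its Box, it saves the player's current location, rather than its own, into the player's Respawn variable on every overlap.
; If ShowText is enabled, a DoOnce shows the UI_CheckpointReached widget the first time only and removes it after a short delay.
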(event `self.Box.OnComponentBeginOverlap`
  (params (OverlappedComponent :type "PrimitiveComponent Object Reference") (OtherActor :type "Actor Object Reference") (OtherComp :type "PrimitiveComponent Object Reference") (OtherBodyIndex :type Integer) (bFromSweep :type Boolean) (SweepResult :type "HitResult Structure (by ref)"))
  (bind _asbp_player (cast `/Game/_Blueprints/Player/BP_Player` OtherActor))
  (set `/Game/_Blueprints/Player/BP_Player.Respawn` (`self.K2_GetActorLocation` _asbp_player) _asbp_player)
  (if (`self.ShowText?`)
    (`/Engine/EditorBlueprintResources/StandardMacros.DoOnce` false
      (:`Completed`
        (bind _returnvalue (`|CreateWidget` "/Game/_UI/UI_CheckpointReached.UI_CheckpointReached_C" (`GameplayStatics.GetPlayerController` 0)))
        (`UserWidget.AddToViewport` _returnvalue 0)
        (`KismetSystemLibrary.Delay` 3.0)
        (`Widget.RemoveFromParent` _returnvalue)))))

(fn `UserConstructionScript`)