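; Game mode Blueprint that handles the player being caught, using the destruction of BP_Player as the trigger.
; BeginPlay and the Respawn event both bind OnCaught to the player character's OnDestroyed delegate.
; OnCaught teleports the destroyed actor to the stored SpawnTransform location, calls Respawn to rebind and plays the FadeIn level sequence.
; No new pawn is spawned in this graph.
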(event `Respawn`
  (bind _asbp_player (cast `/Game/_Blueprints/Player/BP_Player` (`GameplayStatics.GetPlayerCharacter` 0) :!label _label))
  (add `self.OnDestroyed` _asbp_player (delegate `OnCaught`)))

(event `self.ReceiveBeginPlay`
  (goto _label))

(event `OnCaught` :!signature `self.OnDestroyed`
  (params (DestroyedActor :type "Actor Object Reference"))
  (bind _spawn_transform_location (`KismetMathLibrary.BreakTransform` (`self.Spawn Transform`)))
  (`self.K2_SetActorLocation` DestroyedActor _spawn_transform_location false true)
  (`self.Respawn`)
  (bind _outactor (`LevelSequencePlayer.CreateLevelSequencePlayer` "/Game/_LevelSequence/FadeIn.FadeIn"))
  (`MovieSceneSequencePlayer.Play` (`LevelSequenceActor.SequencePlayer` _outactor)))

(fn `UserConstructionScript`)