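; Hackable computer that the player hacks by holding Interact inside its trigger box, opening a linked gate and powering a wire.
; The box overlap toggles input and the UI_Hack widget, with a Gate node limiting when presses count.
; A retriggerable delay checks that the key is still held before a DoOnce fires completion.
; A separate timer, polled by a self-calling delay loop, feeds the widget's progress bar.
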(event `InputAction|Interact`
  (params (Key :type "Key Structure"))
  (bind _canbehacked (`self.canBeHacked`))
  (:`Pressed`
    (if _canbehacked
      (set `self.IsHeld?` true)
      (`/Engine/EditorBlueprintResources/StandardMacros.Gate` true :!label _label
        (:`Exit`
          (`|ExecutionSequence`
            (:`then_0`
              (`KismetSystemLibrary.RetriggerableDelay` (`self.MaxHoldTime`))
              (if (`self.IsHeld?`)
                (set `self.IsHacked?` true)
                (`/Engine/EditorBlueprintResources/StandardMacros.DoOnce` false :!label _label_2
                  (:`Completed`
                    (`GameplayStatics.SpawnSoundAtLocation` "/Game/_Sounds/Hacking/Complete/Hack_Complete_2.Hack_Complete_2" (0.0 0.0 0.0) (struct) 0.2 1.0 0.0 null null)
                    (`/Game/_Blueprints/BP_Gate.Slide Door Open` (`self.GateRef`))
                    (`/Game/_Blueprints/BP_WireSpline.Powered` (`self.Wire`))))))
            (:`then_1`
              (`self.Timer`)
              (`self.Update Timer`)))))))
  (:`Released`
    (if _canbehacked
      (set `self.IsHeld?` false))))

(event `self.Box.OnComponentBeginOverlap`
  (params (OverlappedComponent :type "PrimitiveComponent Object Reference") (OtherActor :type "Actor Object Reference") (OtherComp :type "PrimitiveComponent Object Reference") (OtherBodyIndex :type Integer) (bFromSweep :type Boolean) (SweepResult :type "HitResult Structure (by ref)"))
  (cast `/Game/_Blueprints/BP_Player` OtherActor)
  (if (`self.canBeHacked`)
    (`self.EnableInput` (`GameplayStatics.GetPlayerController` 0))
    (bind _returnvalue (`|CreateWidget` "/Game/_UI/UI_Hack.UI_Hack_C"))
    (bind _output_get (set `self.WidgetRef` _returnvalue))
    (`UserWidget.AddToViewport` _output_get 0)
    (set `/Game/_UI/UI_Hack.MaxTimeHeld` (`self.MaxHoldTime`) _output_get)
    (if (`self.IsHacked?`)
      (`self.DisableInput` (`GameplayStatics.GetPlayerController` 0))
      (`Widget.RemoveFromParent` _returnvalue)
      (goto _label_2)
      (else
        (goto _label :!via `Open`)))))

(event `self.Box.OnComponentEndOverlap`
  (params (OverlappedComponent :type "PrimitiveComponent Object Reference") (OtherActor :type "Actor Object Reference") (OtherComp :type "PrimitiveComponent Object Reference") (OtherBodyIndex :type Integer))
  (cast `/Game/_Blueprints/BP_Player` OtherActor)
  (if (`self.canBeHacked`)
    (`self.DisableInput` (`GameplayStatics.GetPlayerController` 0))
    (`Widget.RemoveFromParent` (stale `self.Box.OnComponentBeginOverlap` _returnvalue))
    (if (`self.IsHacked?`)
      (`self.DisableInput` (`GameplayStatics.GetPlayerController` 0))
      (`Widget.RemoveFromParent` (stale `self.Box.OnComponentBeginOverlap` _returnvalue))
      (else
        (goto _label :!via `Close`)))))

(event `Stop Timer`
  ;[1 1 1] Update Hacking Bar
  (`KismetSystemLibrary.K2_PauseTimerHandle` (stale `Timer` _returnvalue)))

(event `Timer`
  ;[1 1 1] Update Hacking Bar
  (bind _returnvalue (`KismetSystemLibrary.K2_SetTimerDelegate` (delegate `Timer`) (`self.MaxHoldTime`))))

(event `Update Timer`
  (bind _widgetref (`self.WidgetRef`))
  ;[1 1 1] Update Hacking Bar
  (if (`self.IsHeld?`)
    (set `/Game/_UI/UI_Hack.TimeHeld` (`KismetSystemLibrary.K2_GetTimerElapsedTimeHandle` (stale `Timer` _returnvalue)) _widgetref)
    (else
      (`self.Stop Timer`)
      (set `/Game/_UI/UI_Hack.TimeHeld` 0.0 _widgetref)))
  (`KismetSystemLibrary.Delay` 0.005)
  (`self.Update Timer`))

(fn `UserConstructionScript`)