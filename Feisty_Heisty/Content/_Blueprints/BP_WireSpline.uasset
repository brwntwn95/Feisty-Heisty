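; Spline-based wire actor that shows a powered or unpowered state through its material colour and emissive glow.
; The construction script tiles PlacedMesh along the spline as instanced static meshes, spaced by mesh X bounds plus MeshOffset, each rotated toward the next point.
; BeginPlay calls the Powered or Unpowered event from IsPowered, setting material parameters on the instanced mesh component.
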(event `self.ReceiveBeginPlay`
  (if (`self.isPowered?`)
    (`self.Powered`)
    (else
      (`self.Unpowered`))))

(event `Unpowered`
  (bind _instancedstaticmesh (`self.InstancedStaticMesh`))
  (`MeshComponent.SetVectorParameterValueOnMaterials` _instancedstaticmesh "WireColour" (0.15 0.15 0.05))
  (`MeshComponent.SetScalarParameterValueOnMaterials` _instancedstaticmesh "Emissive" 0.5))

(event `Powered`
  (bind _instancedstaticmesh (`self.InstancedStaticMesh`))
  (`MeshComponent.SetVectorParameterValueOnMaterials` _instancedstaticmesh "WireColour" (1.2 1.2 0.4))
  (`MeshComponent.SetScalarParameterValueOnMaterials` _instancedstaticmesh "Emissive" 20.0))

(fn `Get Location At Index`
  (params (A :type Integer))
  (returns (ReturnValue :type "Vector Structure"))
  (return (`SplineComponent.GetLocationAtDistanceAlongSpline` (`self.Spline`) (* A (`self.Spacing`)) "Local")))

(fn `UserConstructionScript`
  (locals (NumberOfInstances :type Integer :default 0))
  (bind (_min _max) (break `Box` (`StaticMesh.GetBoundingBox` (`self.PlacedMesh`))))
  (`StaticMeshComponent.SetStaticMesh` (`self.InstancedStaticMesh`) (`self.PlacedMesh`))
  ;[1 1 1] Tile Next Mesh
  (bind _output_get (set `self.Spacing` (+ (.x (- _max _min)) (`self.MeshOffset`))))
  (bind _output_get_2 (set `local.NumberOfInstances` (`KismetMathLibrary.FFloor` (/ (`SplineComponent.GetSplineLength` (`self.Spline`)) _output_get))))
  (for _index (range (+ _output_get_2 1))
    (bind _returnvalue (`self.Get Location At Index` _index))
    (`InstancedStaticMeshComponent.AddInstance` (`self.InstancedStaticMesh`) (`KismetMathLibrary.MakeTransform` _returnvalue (`KismetMathLibrary.MakeRotFromX` (- (`self.Get Location At Index` (+ _index 1)) _returnvalue))) false)))