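; Enemy security camera that sweeps between two yaw limits and catches the player on sight.
; RotateCam starts on BeginPlay and loops MoveComponentTo, with a FlipFlop switching the target between low and max offsets from the root's yaw.
; When the view cone overlaps the player's dedicated camera collider, it calls PlayerCaught on the cached player and plays an alarm.
; A DoOnce with a delayed reset throttles repeat detections.
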(event `self.ViewCone_0.OnComponentBeginOverlap`
  (params (OverlappedComponent :type "PrimitiveComponent Object Reference") (OtherActor :type "Actor Object Reference") (OtherComp :type "PrimitiveComponent Object Reference") (OtherBodyIndex :type Integer) (bFromSweep :type Boolean) (SweepResult :type "HitResult Structure (by ref)"))
  ;[1 1 1 1 50] Camera Collider Detection / Set Player Reference & Start Camera rotation
  (if (`PrimitiveComponent.IsOverlappingComponent` (`/Game/_Blueprints/Player/BP_Player.ColliderForCamera` (`self.PlayerREF`)) OtherComp)
    (`/Engine/EditorBlueprintResources/StandardMacros.DoOnce` false :!label _label
      (:`Completed`
        (`/Game/_Blueprints/Player/BP_Player.Player Caught` (`self.PlayerREF`))
        (`GameplayStatics.PlaySoundAtLocation` "/Game/_Sounds/Alarms/Camera_Alarm_Cue.Camera_Alarm_Cue" (`self.Camera World Location`) (struct) 0.8 1.0 0.0 null null null null)
        (`KismetSystemLibrary.Delay` 2.5)
        (goto _label :!via `Reset`)))))

(event `self.ReceiveBeginPlay`
  ;[1 1 1 1 50] Camera Collider Detection / Set Player Reference & Start Camera rotation
  (`self.Rotate Cam`)
  (bind _asbp_player (cast `/Game/_Blueprints/Player/BP_Player` (`GameplayStatics.GetPlayerCharacter` 0)))
  (set `self.PlayerREF` _asbp_player))

(event `Rotate Cam`
  (bind (_world_location _set_rotation _rot_speed _camera) (`self.Camera Rotation`))
  ;[1 1 1 1 50] Rotate Camera
  (`/Engine/EditorBlueprintResources/StandardMacros.FlipFlop` :!label _label_2
    (:`A`
      (set `self.Reached One of the sides` true))
    (:`B`
      (set `self.Reached One of the sides` false)))
  (`KismetSystemLibrary.MoveComponentTo` _camera _world_location _set_rotation false false _rot_speed true)
  (goto _label_2))

(fn `UserConstructionScript`)