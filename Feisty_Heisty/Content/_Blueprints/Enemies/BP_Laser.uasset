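; BP_Laser is a rotating laser enemy that detects when its beam crosses the player.
; Each tick it line traces 500 units forward from its Arrow component and spins the actor in yaw by RotationSpeed, scaled by delta time.
; A hit on BP_Player only prints a message, gated by a DoOnce that resets after a one-second delay.
; The trace has no debug drawing, and no damage is applied.
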(event `self.ReceiveTick`
  (params (DeltaSeconds :type "Float (single-precision)"))
  (bind _arrow (`self.Arrow`))
  (bind _returnvalue (`SceneComponent.K2_GetComponentLocation` _arrow))
  ;[1 0.7067 0.6868] Draws a line and detects if player was hit
  (bind _outhit (`KismetSystemLibrary.LineTraceSingleByProfile` _returnvalue (+ _returnvalue (* (`SceneComponent.GetForwardVector` _arrow) 500.0))))
  (`self.K2_AddActorLocalRotation` (* (`KismetMathLibrary.MakeRotator` 0.0 0.0 (`self.Rotation Speed`)) DeltaSeconds))
  (cast `/Game/_Blueprints/Player/BP_Player` (`.HitActor` (`GameplayStatics.BreakHitResult` _outhit)))
  (`/Engine/EditorBlueprintResources/StandardMacros.DoOnce` false :!label _label
    (:`Completed`
      (`KismetSystemLibrary.PrintText` "Hit by Laser!")
      (`KismetSystemLibrary.Delay` 1.0)
      (goto _label :!via `Reset`))))

(fn `UserConstructionScript`)