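; BP_Fireplace is a fireplace actor whose point light flickers during play.
; BeginPlay starts the Flickering timeline, whose updates each move the light's intensity halfway from its current value toward a target, smoothing the changes.
; The same update feeds a randomly timed Delay that then picks a new random target intensity within a narrow range, giving an irregular flicker.
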(event `self.ReceiveBeginPlay`
  (bind _pointlight (`self.PointLight`))
  (`Timeline|Flickering`
    (:`Update`
      (`|ExecutionSequence`
        (:`then_0`
          (`LightComponent.SetIntensity` _pointlight (`KismetMathLibrary.Lerp` (`LightComponentBase.Intensity` _pointlight) (`self.TargetIntensity`) 0.5)))
        (:`then_1`
          (`KismetSystemLibrary.Delay` (`KismetMathLibrary.RandomFloatInRange` 0.1 0.5))
          (set `self.TargetIntensity` (`KismetMathLibrary.RandomFloatInRange` 4.0 6.0)))))))

(fn `UserConstructionScript`)